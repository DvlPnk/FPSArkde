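; BP_Character is a character Blueprint that sets up the player's HUD, camera view and ultimate-ability screen effect.
; BeginPlay adds BP_MainHUD to the viewport and caches the normal post-process settings.
; StartUltimate and StopUltimate swap between ultimate and normal post-process settings, while GainUltimateXP only prints the amount.
; The construction script sets auto-activation of the first-person camera and right third-person camera with spring arm from view flags.
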(event EventBeginPlay
  (Utilities|FlowControl|Sequence
    (:then_0
      (bind _returnvalue (UserInterface|CreateWidget "/Game/Blueprints/UI/HUD/BP_MainHUD.BP_MainHUD_C"))
      (UserInterface|Viewport|AddtoViewport _returnvalue 0))
    (:then_1
      (Variables|Default|SetNormalPostProcess (Variables|/Script/Engine.PostProcessComponent|GetSettings (Variables|Default|GetPostProcess))))))

(event EventGainUltimateXP
  (params (XPGained :type Float%20%28single-precision%29))
  (Development|PrintString (Utilities|String|ToString(Float) XPGained)))

(event EventStartUltimate
  (Variables|/Script/Engine.PostProcessComponent|SetSettings (Variables|Default|GetPostProcess) (Variables|Default|GetUltimatePostProcess)))

(event EventStopUltimate
  (Variables|/Script/Engine.PostProcessComponent|SetSettings (Variables|Default|GetPostProcess) (Variables|Default|GetNormalPostProcess)))

(fn ConstructionScript
  (Components|Activation|SetAutoActivate (Variables|Default|GetFPSCameraComponent) (Variables|Default|GetbUseFirstPersonView))
  (Components|Activation|SetAutoActivate (Variables|Default|GetTPSCameraComponent_R) (Variables|Default|GetbUseTPersonView_R)))